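; BP_MultiGoal is a goal that destroys an assigned object once a required number of balls have hit it.
; On Hit, it removes the first tag of any actor tagged "Ball", normally so that ball counts only once, and increments BallsInGoal.
; CheckGoal then destroys ObjectToRemove, if valid, when the count exactly equals BallsRequired.
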(event Custom|CheckGoal
  (bind _objecttoremove (Variables|Default|GetObjectToRemove))
  (if (== (Variables|Default|GetBallsRequired) (Variables|Default|GetBallsInGoal))
    (Utilities|IsValid _objecttoremove
      (:Is%20Valid
        (Actor|DestroyActor _objecttoremove)))))

(event Collision|EventHit
  (params (MyComp :type Primitive%20Component%20Object%20Reference) (Other :type Actor%20Object%20Reference) (OtherComp :type Primitive%20Component%20Object%20Reference) (bSelfMoved :type Boolean) (HitLocation :type Vector :default "0, 0, 0") (HitNormal :type Vector :default "0, 0, 0") (NormalImpulse :type Vector :default "0, 0, 0") (Hit :type Hit%20Result%20Structure%20%28by%20ref%29))
  (if (Actor|ActorHasTag Other "Ball")
    (Utilities|Array|RemoveIndex (Variables|/Script/Engine.Actor|GetTags Other))
    (bind _output_get (Variables|Default|SetBallsInGoal (Variables|Default|GetBallsInGoal)))
    (Math|Integer|IncrementInt _output_get
      (:%20%20
        (CallFunction|CheckGoal)))))

(fn ConstructionScript)