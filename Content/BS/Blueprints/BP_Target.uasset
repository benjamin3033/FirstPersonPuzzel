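; BP_Target is a shootable target actor that reacts only to hits from a FirstPersonProjectile.
; On a hit it sets BeenHit and, if an ObjectToDestroy is assigned, destroys that linked actor after a delay.
; It then either removes itself after a second delay or stays, optionally halting its InterpToMovement component, as chosen by the RemoveTargetOnHit and StopMovementOnHit flags.
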(event Collision|EventHit
  (params (MyComp :type Primitive%20Component%20Object%20Reference) (Other :type Actor%20Object%20Reference) (OtherComp :type Primitive%20Component%20Object%20Reference) (bSelfMoved :type Boolean) (HitLocation :type Vector :default "0, 0, 0") (HitNormal :type Vector :default "0, 0, 0") (NormalImpulse :type Vector :default "0, 0, 0") (Hit :type Hit%20Result%20Structure%20%28by%20ref%29))
  (Utilities|Casting|CastToFirstPersonProjectile Other)
  (Variables|Default|SetBeenHit true)
  (Utilities|IsValid (Variables|Default|GetObjectToDestroy)
    (:Is%20Valid
      (Utilities|FlowControl|Delay (Variables|Default|GetDelayBeforeObjectRemoval))
      (Actor|DestroyActor (Variables|Default|GetObjectToDestroy)))
    (:Is%20Not%20Valid
      _))
  (if (Variables|Default|GetRemoveTargetOnHit)
    (Utilities|FlowControl|Delay (Variables|Default|GetDelayBeforeTargetRemoval))
    (Actor|DestroyActor)
    (elif (Variables|Default|GetStopMovementOnHit)
      (Components|Activation|Deactivate (Variables|Default|GetInterpToMovement)))))

(fn ConstructionScript)